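; Player-controllable tank Blueprint that wires input to C++-style Aiming and Movement components and sets up a health bar widget.
; On BeginPlay it passes barrel, turret and tracks to those components and gives the HealthBar widget a reference to itself.
; Movement axes feed Movement intents, aim axes rotate the gimbal and spring arm, Fire triggers Aiming, and SwapCam toggles first and third person cameras.
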(event `self.ReceiveBeginPlay`
  (`TankAimingComponent.Initialize` (`self.Aiming`) (`self.Barrel`) (`self.Turret`))
  (`TankMovementComponent.Initialize` (`self.Movement`) (`self.LeftTrack`) (`self.RightTrack`))
  (`self.InitialiseHealthBarWidget`))

(event `InputAxis|AimAzimuth`
  (params (AxisValue :type "Float (single-precision)"))
  ;[1 1 1] Input Aim Binding
  (`SceneComponent.K2_AddLocalRotation` (`self.Gimball`) (`KismetMathLibrary.MakeRotator` 0.0 0.0 AxisValue) false false))

(event `InputAxis|MoveForward`
  (params (AxisValue :type "Float (single-precision)"))
  ;[1 1 1] Movement Input Binding
  (`TankMovementComponent.IntendMoveForward` (`self.Movement`) AxisValue))

(event `InputAxis|TurnRight`
  (params (AxisValue :type "Float (single-precision)"))
  ;[1 1 1] Movement Input Binding
  (`TankMovementComponent.IntendTurnRight` (`self.Movement`) AxisValue))

(event `InputAxis|AimElevation`
  (params (AxisValue :type "Float (single-precision)"))
  ;[1 1 1] Input Aim Binding
  (`SceneComponent.K2_AddLocalRotation` (`self.SpringArm`) (`KismetMathLibrary.MakeRotator` 0.0 AxisValue) false false))

(event `InputAction|Fire`
  (params (Key :type "Key Structure"))
  ;[1 1 1] Input Aim Binding
  (:`Pressed`
    (`TankAimingComponent.Fire` (`self.Aiming`))))

(event `InputAction|SwapCam`
  (params (Key :type "Key Structure"))
  ;[1 1 1] Camera Swapping
  (:`Pressed`
    (`ActorComponent.ToggleActive` (`self.FirstPersonCamera`))
    (`ActorComponent.ToggleActive` (`self.ThirdPersonCamera`))))

(fn `InitialiseHealthBarWidget`
  (bind _ashealth_bar (cast `/Game/Widgets/HealthBar` (`WidgetComponent.GetUserWidgetObject` (`self.HealthBar`))))
  (set `/Game/Widgets/HealthBar.MyTank` self _ashealth_bar))

(fn `UserConstructionScript`)